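; TTPlayerController_BP is a player controller that holds a debug check for ModelStats_UMG widgets.
; Pressing B prints a confirmation, gathers all widgets of that class, including non-top-level ones, and prints their count.
; An unconnected loop meant to print details of each found widget never runs, and BeginPlay, Tick and the construction script are empty.
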(event `Key|B`
  (params (Key :type "Key Structure"))
  (:`Pressed`
    (`KismetSystemLibrary.PrintString` "B Pressed")
    (bind _foundwidgets (`WidgetBlueprintLibrary.GetAllWidgetsOfClass` "/Game/UI/ModelStats_UMG.ModelStats_UMG_C" false))
    (`KismetSystemLibrary.PrintString` (`KismetStringLibrary.Conv_IntToString` (`KismetArrayLibrary.Array_Length` _foundwidgets)))))

(event `self.ReceiveBeginPlay`)

(event `self.ReceiveTick`
  (params (DeltaSeconds :type "Float (single-precision)")))

(fn `UserConstructionScript`)